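; BP_Projectile is a projectile that scores points for the player when it overlaps an enemy.
; Tick moves it along world X at ProjectileSpeed, scaled by delta time.
; Sphere overlaps with BP_enemy call AddScore on the BP_Player pawn and destroy the projectile, while overlaps with BP_Tunnel or any component hit only destroy it.
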(event OnComponentHit(Sphere)
  (params (HitComponent :type Primitive%20Component%20Object%20Reference) (OtherActor :type Actor%20Object%20Reference) (OtherComp :type Primitive%20Component%20Object%20Reference) (NormalImpulse :type Vector :default "0, 0, 0") (Hit :type Hit%20Result%20Structure%20%28by%20ref%29))
  (Actor|DestroyActor))

(event OnComponentBeginOverlap(Sphere)
  (params (OverlappedComponent :type Primitive%20Component%20Object%20Reference) (OtherActor :type Actor%20Object%20Reference) (OtherComp :type Primitive%20Component%20Object%20Reference) (OtherBodyIndex :type Integer) (bFromSweep :type Boolean) (SweepResult :type Hit%20Result%20Structure%20%28by%20ref%29))
  (Utilities|FlowControl|Sequence
    (:then_0
      (Utilities|Casting|CastToBP_enemy OtherActor)
      (bind _asbp_player (Utilities|Casting|CastToBP_Player (Game|Player|GetPlayerPawn 0)))
      (Default|AddScore _asbp_player))
    (:then_1
      (Utilities|Casting|CastToBP_Tunnel OtherActor)))
  (Actor|DestroyActor))

(event EventBeginPlay
  (Utilities|Casting|CastToBP_Player (Game|Player|GetPlayerPawn 0)))

(event Collision|EventActorBeginOverlap
  (params (OtherActor :type Actor%20Object%20Reference)))

(event EventTick
  (params (DeltaSeconds :type Float%20%28single-precision%29))
  (Transformation|AddActorWorldOffset (Math|Vector|MakeVector (* DeltaSeconds (Variables|Default|GetProjectileSpeed)) 0.0 0.0)))

(fn ConstructionScript)